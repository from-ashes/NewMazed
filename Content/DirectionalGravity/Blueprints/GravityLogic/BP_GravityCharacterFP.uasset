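; First-person directional-gravity player character that handles level intro, dashing, death, restart, pause and the EndGame credits key.
; BeginPlay fades in audio and tints the world's edge effect red or blue by level name.
; Outside Start, staying airborne about three seconds spawns DeathBP ahead, pulls the player into it, then loads the level's "_red" variant (Start from EndGame).
; A timed gate makes Dash a double-tap impulse along camera forward.
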(event `self.ReceiveBeginPlay`
  (bind _audio (`self.Audio`))
  (`AudioComponent.SetVolumeMultiplier` _audio 0.0)
  (bind (_direction _newtrack_0) (`Timeline|Timeline_0` :!via `PlayFromStart`)
    (:`Update`
      (`AudioComponent.SetVolumeMultiplier` _audio _newtrack_0)
      (`/Engine/EditorBlueprintResources/StandardMacros.DoOnce` false
        (:`Completed`
          (`WidgetBlueprintLibrary.SetInputMode_GameOnly` (`GameplayStatics.GetPlayerController` 0))
          (set `self.LevelComplete` true)
          (`KismetMaterialLibrary.SetScalarParameterValue` "/Game/Assets/WorldCollection.WorldCollection" "EdgeEffectToggle" 1.0)
          (bind _returnvalue (`GameplayStatics.GetCurrentLevelName` true))
          (if (`KismetStringLibrary.Contains` _returnvalue "Red")
            (`KismetMaterialLibrary.SetScalarParameterValue` "/Game/Assets/WorldCollection.WorldCollection" "R" 1.0)
            (`KismetMaterialLibrary.SetScalarParameterValue` "/Game/Assets/WorldCollection.WorldCollection" "G")
            (`KismetMaterialLibrary.SetScalarParameterValue` "/Game/Assets/WorldCollection.WorldCollection" "B")
            (else
              (`KismetMaterialLibrary.SetScalarParameterValue` "/Game/Assets/WorldCollection.WorldCollection" "R")
              (`KismetMaterialLibrary.SetScalarParameterValue` "/Game/Assets/WorldCollection.WorldCollection" "G" -0.163033)
              (`KismetMaterialLibrary.SetScalarParameterValue` "/Game/Assets/WorldCollection.WorldCollection" "B" 1.0))))))))

(event `self.ReceiveTick`
  (params (DeltaSeconds :type "Float (single-precision)"))
  (bind _isonground (`self.IsOnGround`))
  (`parent.ReceiveTick` DeltaSeconds)
  (`KismetSystemLibrary.Delay` 0.2)
  (bind _returnvalue (`GameplayStatics.GetCurrentLevelName` true))
  (if (`KismetStringLibrary.EqualEqual_StrStr` _returnvalue "Start")
    _
    (elif (not _isonground)
      (`KismetSystemLibrary.Delay` 3.0)
      (if (not _isonground)
        (`self.DeathEvent`)))))

(event `Teleporting`
  (bind (_direction _newtrack_0) (`Timeline|Timeline_1` :!via `PlayFromStart`)
    (:`Update`
      (set `CameraComponent.FieldOfView` _newtrack_0 (`self.Camera`)))))

(event `Key|H`
  (params (Key :type "Key Structure"))
  (:`Pressed`
    (bind _returnvalue (`GameplayStatics.GetCurrentLevelName` true))
    (if (`KismetStringLibrary.EqualEqual_StrStr` _returnvalue "EndGame")
      (bind _foundwidgets (`WidgetBlueprintLibrary.GetAllWidgetsOfClass` "/Game/UI/Credits.Credits_C"))
      (`/Game/UI/Credits.Animate` (`|GetArrayItem` _foundwidgets)))))

(event `DeathEvent`
  (bind _camera (`self.Camera`))
  (bind _walkcollision (`self.WalkCollision`))
  (`/Engine/EditorBlueprintResources/StandardMacros.DoOnce` false
    (:`Completed`
      (bind _returnvalue (`|SpawnActorFromClass` "/Game/Assets/DeathActionBP/DeathBP.DeathBP_C" (`KismetMathLibrary.MakeTransform` (+ (`SceneComponent.K2_GetComponentLocation` _camera) (* (`SceneComponent.GetForwardVector` _camera) 1000.0))) "AlwaysSpawn" "OverrideRootScale" null null))
      (bind (_direction _newtrack_0) (`Timeline|Timeline_2` :!via `PlayFromStart`)
        (:`Update`
          (`SceneComponent.K2_SetWorldLocation` _walkcollision (`KismetMathLibrary.VLerp` (`SceneComponent.K2_GetComponentLocation` _walkcollision) (`SceneComponent.K2_GetComponentLocation` (`/Game/Assets/DeathActionBP/DeathBP.DefaultSceneRoot` _returnvalue)) _newtrack_0) false false))
        (:`Finished`
          (bind _returnvalue_2 (`GameplayStatics.GetCurrentLevelName` true))
          (if (`KismetStringLibrary.EqualEqual_StrStr` _returnvalue_2 "EndGame")
            (`GameplayStatics.OpenLevel` "Start")
            (else
              (`GameplayStatics.OpenLevel` (`KismetStringLibrary.Conv_StringToName` (`KismetStringLibrary.Concat_StrStr` _returnvalue_2 "_red"))))))))))

(event `InputAction|Pause`
  (params (Key :type "Key Structure"))
  (:`Pressed`
    (bind _returnvalue (`|CreateWidget` "/Game/UI/PauseMenu.PauseMenu_C"))
    (`UserWidget.AddToViewport` _returnvalue 0)))

(event `InputAction|Restart`
  (params (Key :type "Key Structure"))
  (:`Pressed`
    (bind _returnvalue (`GameplayStatics.GetCurrentLevelName` true))
    (`GameplayStatics.OpenLevel` (`KismetStringLibrary.Conv_StringToName` _returnvalue))))

(event `InputAction|Dash`
  (params (Key :type "Key Structure"))
  (:`Pressed`
    (`|ExecutionSequence`
      (:`then_0`
        (`/Engine/EditorBlueprintResources/StandardMacros.Gate` true :!label _label
          (:`Exit`
            (`PrimitiveComponent.AddImpulse` (`self.WalkCollision`) (* (`KismetMathLibrary.Normal` (`SceneComponent.GetForwardVector` (`self.Camera`))) (`self.DashStrength`)) "None" true))))
      (:`then_1`
        (goto _label :!via `Open`))
      (:`then_2`
        (`KismetSystemLibrary.Delay` 0.3)
        (goto _label :!via `Close`)))))

(fn `UserConstructionScript`
  (`parent.UserConstructionScript`))