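; MiscObjectBP is a scenery prop that picks a random brick-cluster or gemstone mesh by part type in its construction script, which also clears Floating and Glitching if both are set.
; Floating props follow a timeline toward a random nearby point.
; Glitching Obsidian props use a Tick-fed gate to run three stages of increasingly rapid random jumps, then a timeline scales the mesh and a sphere, reverses, and restarts the cycle.
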(event `self.ReceiveBeginPlay`
  (bind _returnvalue (`KismetMathLibrary.RandomFloatInRange` -50.0 50.0))
  (bind _staticmesh (`self.StaticMesh`))
  (if (`self.Floating?`)
    (set `self.Starting Vector` (`SceneComponent.K2_GetComponentLocation` _staticmesh))
    (bind _output_get (set `self.Random Vector` (`KismetMathLibrary.MakeVector` _returnvalue _returnvalue _returnvalue)))
    (set `self.End Vector` (+ _output_get (`self.Starting Vector`)))
    (bind (_direction _newtrack_0) (`Timeline|Timeline_0`)
      (:`Update`
        (`SceneComponent.K2_SetWorldLocation` _staticmesh (`KismetMathLibrary.VLerp` (`self.Starting Vector`) (`self.End Vector`) _newtrack_0) false false)))))

(event `self.ReceiveTick`
  (params (DeltaSeconds :type "Float (single-precision)"))
  (bind _returnvalue (`KismetMathLibrary.RandomFloatInRange` -10.0 10.0))
  (bind _returnvalue_2 (`KismetMathLibrary.RandomFloatInRange` -10.0 10.0))
  (bind _returnvalue_3 (`KismetMathLibrary.RandomFloatInRange` -10.0 10.0))
  (bind _staticmesh (`self.StaticMesh`))
  (bind _staticmesh_2 (`self.StaticMesh`))
  (bind _staticmesh_3 (`self.StaticMesh`))
  (bind (_returnvalue_x _returnvalue_y _returnvalue_z) (`KismetMathLibrary.BreakVector` (`SceneComponent.K2_GetComponentLocation` _staticmesh)))
  (bind (_returnvalue_x_2 _returnvalue_y_2 _returnvalue_z_2) (`KismetMathLibrary.BreakVector` (`SceneComponent.K2_GetComponentLocation` _staticmesh_2)))
  (bind (_returnvalue_x_3 _returnvalue_y_3 _returnvalue_z_3) (`KismetMathLibrary.BreakVector` (`SceneComponent.K2_GetComponentLocation` _staticmesh_3)))
  (if (`self.Glitching?`)
    (switch `/Game/Assets/Misc/MiscLogic/MiscParts` (`self.MiscPartsEnum`)
      (:`NewEnumerator1`
        (if (`self.FirstFire?`)
          (`KismetSystemLibrary.Delay` (`KismetMathLibrary.RandomFloatInRange` 1.0 25.0))
          (set `self.FirstFire?` false)
          (goto _label :!via `Open`)
          (else
            (`/Engine/EditorBlueprintResources/StandardMacros.Gate` true :!label _label
              (:`Exit`
                (if (`self.Should Delay?`)
                  (`KismetSystemLibrary.Delay` (`self.CycleDelay`)))
                (switch `int` (`self.Cycle`)
                  (:`0`
                    (`KismetSystemLibrary.Delay` (`KismetMathLibrary.RandomFloatInRange` 0.3 0.7))
                    (bind _counter (`/Engine/EditorBlueprintResources/StandardMacros.Do N` (`self.Times To Jump`) :!label _label_2)
                      (:`Exit`
                        (switch `int` (`KismetMathLibrary.RandomIntegerInRange` 0 3)
                          (:`0`
                            (`SceneComponent.K2_SetWorldLocation` _staticmesh_2 (`KismetMathLibrary.MakeVector` (+ _returnvalue_x_2 _returnvalue_2) _returnvalue_y_2 _returnvalue_z_2) false false))
                          (:`1`
                            (`SceneComponent.K2_SetWorldLocation` _staticmesh_2 (`KismetMathLibrary.MakeVector` _returnvalue_x_2 (+ _returnvalue_y_2 _returnvalue_2) _returnvalue_z_2) false false))
                          (:`2`
                            (`SceneComponent.K2_SetWorldLocation` _staticmesh_2 (`KismetMathLibrary.MakeVector` _returnvalue_x_2 _returnvalue_y_2 (+ _returnvalue_z_2 _returnvalue_2)) false false))
                          (:`3`
                            (`SceneComponent.K2_SetWorldLocation` _staticmesh_2 (`KismetMathLibrary.MakeVector` _returnvalue_x_2 _returnvalue_y_2 _returnvalue_z_2) false false)))
                        (if (== _counter (`self.Times To Jump`))
                          (`|ExecutionSequence`
                            (:`then_0`
                              (set `self.Times To Jump` (+ (`self.Times To Jump`) (`KismetMathLibrary.RandomIntegerInRange` -2 2)))
                              (set `self.Cycle` 1)
                              (set `self.CycleDelay` (`KismetMathLibrary.RandomFloatInRange` 5.0 7.0))
                              (`self.Reset Stuff`))
                            (:`then_1`
                              (goto _label_2 :!via `Reset`)))))))
                  (:`1`
                    (`KismetSystemLibrary.Delay` (`KismetMathLibrary.RandomFloatInRange` 0.2 0.5))
                    (bind _counter_2 (`/Engine/EditorBlueprintResources/StandardMacros.Do N` (`self.Times To Jump`) :!label _label_3)
                      (:`Exit`
                        (switch `int` (`KismetMathLibrary.RandomIntegerInRange` 0 2)
                          (:`0`
                            (`SceneComponent.K2_SetWorldLocation` _staticmesh_3 (`KismetMathLibrary.MakeVector` (+ _returnvalue_x_3 _returnvalue_3) _returnvalue_y_3 _returnvalue_z_3) false false))
                          (:`1`
                            (`SceneComponent.K2_SetWorldLocation` _staticmesh_3 (`KismetMathLibrary.MakeVector` _returnvalue_x_3 (+ _returnvalue_y_3 _returnvalue_3) _returnvalue_z_3) false false))
                          (:`2`
                            (`SceneComponent.K2_SetWorldLocation` _staticmesh_3 (`KismetMathLibrary.MakeVector` _returnvalue_x_3 _returnvalue_y_3 (+ _returnvalue_z_3 _returnvalue_3)) false false))
                          (:`3`
                            (`SceneComponent.K2_SetWorldLocation` _staticmesh_3 (`KismetMathLibrary.MakeVector` _returnvalue_x_3 _returnvalue_y_3 _returnvalue_z_3) false false)))
                        (if (== _counter_2 (`self.Times To Jump`))
                          (`|ExecutionSequence`
                            (:`then_0`
                              (set `self.Times To Jump` (+ (`self.Times To Jump`) (`KismetMathLibrary.RandomIntegerInRange` -2 2)))
                              (set `self.Cycle` 2)
                              (set `self.CycleDelay` (`KismetMathLibrary.RandomFloatInRange` 3.0 5.0)))
                            (:`then_1`
                              (goto _label_3 :!via `Reset`)))))))
                  (:`2`
                    (`KismetSystemLibrary.Delay` (`KismetMathLibrary.RandomFloatInRange` 0.05 0.1))
                    (bind _counter_3 (`/Engine/EditorBlueprintResources/StandardMacros.Do N` (`self.Times To Jump`) :!label _label_4)
                      (:`Exit`
                        (switch `int` (`KismetMathLibrary.RandomIntegerInRange` 0 2)
                          (:`0`
                            (`SceneComponent.K2_SetWorldLocation` _staticmesh (`KismetMathLibrary.MakeVector` (+ _returnvalue_x _returnvalue) _returnvalue_y _returnvalue_z) false false))
                          (:`1`
                            (`SceneComponent.K2_SetWorldLocation` _staticmesh (`KismetMathLibrary.MakeVector` _returnvalue_x (+ _returnvalue_y _returnvalue) _returnvalue_z) false false))
                          (:`2`
                            (`SceneComponent.K2_SetWorldLocation` _staticmesh (`KismetMathLibrary.MakeVector` _returnvalue_x _returnvalue_y (+ _returnvalue_z _returnvalue)) false false))
                          (:`3`
                            (`SceneComponent.K2_SetWorldLocation` _staticmesh (`KismetMathLibrary.MakeVector` _returnvalue_x _returnvalue_y _returnvalue_z) false false)))
                        (if (== _counter_3 (`self.Times To Jump`))
                          (`|ExecutionSequence`
                            (:`then_0`
                              (set `self.Times To Jump` (+ (`self.Times To Jump`) (`KismetMathLibrary.RandomIntegerInRange` -2 2)))
                              (set `self.Cycle` 3)
                              (set `self.CycleDelay` (`KismetMathLibrary.RandomFloatInRange` 0.5 2.0)))
                            (:`then_1`
                              (goto _label_4 :!via `Reset`)))))))
                  (:`3`
                    (`/Engine/EditorBlueprintResources/StandardMacros.DoOnce` false :!label _label_5
                      (:`Completed`
                        (`|ExecutionSequence`
                          (:`then_0`
                            (bind (_direction _newtrack_0 _newtrack_2) (`Timeline|Timeline_1` :!label _label_6)
                              (:`Update`
                                (`SceneComponent.SetWorldScale3D` (`self.Sphere`) (`KismetMathLibrary.Conv_DoubleToVector` _newtrack_0))
                                (`SceneComponent.SetWorldScale3D` (`self.StaticMesh`) (`KismetMathLibrary.Conv_DoubleToVector` _newtrack_2))
                                (`/Engine/EditorBlueprintResources/StandardMacros.DoOnce` false :!label _label_7
                                  (:`Completed`
                                    (`KismetSystemLibrary.Delay` 11.0)
                                    (`self.ScaleFinished`)))))))))))))))))))

(event `Reset Stuff`
  (`|ExecutionSequence`
    (:`then_0`
      (goto _label_5 :!via `Reset`))
    (:`then_1`
      (goto _label_7 :!via `Reset`))))

(event `ScaleFinished`
  (`|ExecutionSequence`
    (:`then_0`
      (`|ExecutionSequence`
        (:`then_0`
          (goto _label_6 :!via `Reverse`))))
    (:`then_1`
      (set `self.Cycle` 0)
      (set `self.FirstFire?` true))))

(fn `UserConstructionScript`
  (bind _staticmesh (`self.StaticMesh`))
  (bind _staticmesh_2 (`self.StaticMesh`))
  (if (and (`self.Floating?`) (`self.Glitching?`))
    (bind _output_get (set `self.Glitching?` false))
    (set `self.Floating?` _output_get))
  (switch `/Game/Assets/Misc/MiscLogic/MiscParts` (`self.MiscPartsEnum`)
    (:`NewEnumerator0`
      (switch `int` (`KismetMathLibrary.RandomIntegerInRange` 0 12)
        (:`Default`
          (`StaticMeshComponent.SetStaticMesh` _staticmesh_2 "/Game/Assets/Bricks/Cluster_Objects_Object001.Cluster_Objects_Object001" :!label _label))
        (:`0`
          (goto _label))
        (:`1`
          (`StaticMeshComponent.SetStaticMesh` _staticmesh_2 "/Game/Assets/Bricks/Cluster_Objects_Object002.Cluster_Objects_Object002"))
        (:`2`
          (`StaticMeshComponent.SetStaticMesh` _staticmesh_2 "/Game/Assets/Bricks/Cluster_Objects_Object003.Cluster_Objects_Object003"))
        (:`3`
          (`StaticMeshComponent.SetStaticMesh` _staticmesh_2 "/Game/Assets/Bricks/Cluster_Objects_Object004.Cluster_Objects_Object004"))
        (:`4`
          (`StaticMeshComponent.SetStaticMesh` _staticmesh_2 "/Game/Assets/Bricks/Cluster_Objects_Object005.Cluster_Objects_Object005"))
        (:`5`
          (`StaticMeshComponent.SetStaticMesh` _staticmesh_2 "/Game/Assets/Bricks/Cluster_Objects_Object006.Cluster_Objects_Object006"))
        (:`6`
          (`StaticMeshComponent.SetStaticMesh` _staticmesh_2 "/Game/Assets/Bricks/Cluster_Objects_Object007.Cluster_Objects_Object007"))
        (:`7`
          (`StaticMeshComponent.SetStaticMesh` _staticmesh_2 "/Game/Assets/Bricks/Cluster_Objects_Object008.Cluster_Objects_Object008"))
        (:`8`
          (`StaticMeshComponent.SetStaticMesh` _staticmesh_2 "/Game/Assets/Bricks/Cluster_Objects_Object009.Cluster_Objects_Object009"))
        (:`9`
          (`StaticMeshComponent.SetStaticMesh` _staticmesh_2 "/Game/Assets/Bricks/Cluster_Objects_Object010.Cluster_Objects_Object010"))
        (:`10`
          (`StaticMeshComponent.SetStaticMesh` _staticmesh_2 "/Game/Assets/Bricks/Cluster_Objects_Object011.Cluster_Objects_Object011"))
        (:`11`
          (`StaticMeshComponent.SetStaticMesh` _staticmesh_2 "/Game/Assets/Bricks/Cluster_Objects_Object012.Cluster_Objects_Object012"))
        (:`12`
          (`StaticMeshComponent.SetStaticMesh` _staticmesh_2 "/Game/Assets/Bricks/Cluster_Objects_Object013.Cluster_Objects_Object013"))))
    (:`NewEnumerator1`
      (switch `int` (`KismetMathLibrary.RandomIntegerInRange` 0 12)
        (:`Default`
          (`StaticMeshComponent.SetStaticMesh` _staticmesh "/Game/Assets/Misc/Meshes/Gemstrones_Gemstrone_10.Gemstrones_Gemstrone_10" :!label _label_2))
        (:`0`
          (goto _label_2))
        (:`1`
          (`StaticMeshComponent.SetStaticMesh` _staticmesh "/Game/Assets/Misc/Meshes/Gemstrones_Gemstrone_11.Gemstrones_Gemstrone_11"))
        (:`2`
          (`StaticMeshComponent.SetStaticMesh` _staticmesh "/Game/Assets/Misc/Meshes/Gemstrones_Gemstrone_12.Gemstrones_Gemstrone_12"))
        (:`3`
          (`StaticMeshComponent.SetStaticMesh` _staticmesh "/Game/Assets/Misc/Meshes/Gemstrones_Gemstrone_00.Gemstrones_Gemstrone_00"))
        (:`4`
          (`StaticMeshComponent.SetStaticMesh` _staticmesh "/Game/Assets/Misc/Meshes/Gemstrones_Gemstrone_01.Gemstrones_Gemstrone_01"))
        (:`5`
          (`StaticMeshComponent.SetStaticMesh` _staticmesh "/Game/Assets/Misc/Meshes/Gemstrones_Gemstrone_03.Gemstrones_Gemstrone_03"))
        (:`6`
          (`StaticMeshComponent.SetStaticMesh` _staticmesh "/Game/Assets/Misc/Meshes/Gemstrones_Gemstrone_04.Gemstrones_Gemstrone_04"))
        (:`7`
          (`StaticMeshComponent.SetStaticMesh` _staticmesh "/Game/Assets/Misc/Meshes/Gemstrones_Gemstrone_05.Gemstrones_Gemstrone_05"))
        (:`8`
          (`StaticMeshComponent.SetStaticMesh` _staticmesh "/Game/Assets/Misc/Meshes/Gemstrones_Gemstrone_06.Gemstrones_Gemstrone_06"))
        (:`9`
          (`StaticMeshComponent.SetStaticMesh` _staticmesh "/Game/Assets/Misc/Meshes/Gemstrones_Gemstrone_09.Gemstrones_Gemstrone_09"))
        (:`10`
          (`StaticMeshComponent.SetStaticMesh` _staticmesh "/Game/Assets/Misc/Meshes/Gemstrones_Gemstrone_07.Gemstrones_Gemstrone_07"))
        (:`11`
          (`StaticMeshComponent.SetStaticMesh` _staticmesh "/Game/Assets/Misc/Meshes/Gemstrones_Gemstrone_08.Gemstrones_Gemstrone_08"))))))